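; Main menu actor that bobs its FireBall component up and down.
; BeginPlay caches the fireball's world location as the rest point.
; Each Tick advances a Time value wrapped at TAU and offsets the fireball on Z by a sine of it, scaled by Amplitude.
; Speed multiplies the whole accumulated Time each frame, not just the delta, so it is not a linear rate control.
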(event `self.ReceiveBeginPlay`
  (set `self.FireBallStartLoc` (`SceneComponent.K2_GetComponentLocation` (`self.FireBall`))))

(event `self.ReceiveTick`
  (params (DeltaSeconds :type "Float (single-precision)"))
  (bind _output_get (set `self.Time` (mod (* (+ DeltaSeconds (`self.Time`)) (`self.Speed`)) (`KismetMathLibrary.GetTAU`))))
  (`SceneComponent.K2_SetWorldLocation` (`self.FireBall`) (+ (`self.FireBallStartLoc`) (`KismetMathLibrary.MakeVector` 0.0 0.0 (* (`KismetMathLibrary.Sin` _output_get) (`self.Amplitude`)))) false false))

(fn `UserConstructionScript`)