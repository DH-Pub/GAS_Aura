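; BP_Player is the Aura player character Blueprint, holding a few key bindings on top of its parent class.
; Left Ctrl asks the ability system component to activate abilities tagged Ability.Cooldown.Reduce, while G directly plays the Fire Bolt cast montage on the mesh.
; Fade in and out calls through BI_Fade, gated on local control, are left unconnected and never run.
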(event `Key|LeftControl`
  (params (Key :type "Key Structure"))
  (:`Pressed`
    (`AbilitySystemComponent.TryActivateAbilitiesByTag` (`AbilitySystemBlueprintLibrary.GetAbilitySystemComponent` null) (`BlueprintGameplayTagLibrary.MakeGameplayTagContainerFromTag` (struct :`TagName` "Ability.Cooldown.Reduce")) true)))

(event `Key|G`
  (params (Key :type "Key Structure"))
  (:`Pressed`
    (`|PlayMontage` (`self.Mesh`) "/Game/Blueprints/Character/Aura/AM_Cast_FireBolt.AM_Cast_FireBolt")))

(fn `UserConstructionScript`)