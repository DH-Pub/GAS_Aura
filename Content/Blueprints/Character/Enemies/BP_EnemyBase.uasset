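; BP_EnemyBase is the base enemy Blueprint, handling spawn and dissolve visual effects.
; On BeginPlay it disables actor tick and plays a timeline that scales the mesh uniformly, snapping it to full size when finished.
; Two events take a dynamic material instance and drive its Dissolve scalar parameter through separate timelines, one general and one for the weapon.
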(event `self.ReceiveBeginPlay`
  (`self.SetActorTickEnabled` false)
  (bind (_direction _scale) (`Timeline|Spawn`)
    (:`Update`
      (`SceneComponent.SetRelativeScale3D` (`self.Mesh`) (`KismetMathLibrary.MakeVector` _scale _scale _scale)))
    (:`Finished`
      (`SceneComponent.SetRelativeScale3D` (`self.Mesh`) (1.0 1.0 1.0)))))

(event `self.StartDissolveTimeline`
  (params (MIDynamic :type "MaterialInstanceDynamic Object Reference"))
  (bind (_direction _dissolve) (`Timeline|DissolveTimeline`)
    (:`Update`
      (`MaterialInstanceDynamic.SetScalarParameterValue` MIDynamic "Dissolve" _dissolve))))

(event `self.StartWeaponDissolveTimeline`
  (params (MIDynamic :type "MaterialInstanceDynamic Object Reference"))
  (bind (_direction _dissolve) (`Timeline|WeaponDissolveTimeline`)
    (:`Update`
      (`MaterialInstanceDynamic.SetScalarParameterValue` MIDynamic "Dissolve" _dissolve))))

(fn `UserConstructionScript`)