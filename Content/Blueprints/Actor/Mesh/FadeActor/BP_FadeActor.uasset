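; BP_FadeActor is a mesh actor that fades out and back in through its materials.
; Its construction script caches the mesh's original materials and builds dynamic instances from a list of fade materials.
; FadeOut swaps in those instances and plays a timeline driving their "Fade" scalar, while Fadein reverses it.
; When the timeline finishes with intensity at one or above, the original materials are restored.
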(event `/Game/Blueprints/Actor/Mesh/FadeActor/BI_Fade.FadeOut`
  (`self.UpdateMaterials` (`self.DynamicMI`))
  (bind (_direction _intensity) (`Timeline|Fade` :!label _label)
    (:`Update`
      (for _array_element (`self.DynamicMI`)
        (`MaterialInstanceDynamic.SetScalarParameterValue` _array_element "Fade" _intensity)))
    (:`Finished`
      (if (>= _intensity 1.0)
        (`self.UpdateMaterials` (`self.OriginalMaterials`)) ; Reset Material to Default
      ))))

(event `/Game/Blueprints/Actor/Mesh/FadeActor/BI_Fade.FadeIn`
  (goto _label :!via `Reverse`))

(fn `UpdateMaterials`
  (params (Array :type "Array of MaterialInterface Object Reference"))
  (for (_array_element _array_index) Array
    (`PrimitiveComponent.SetMaterial` (`self.Mesh`) _array_index _array_element)))

(fn `UserConstructionScript`
  (`KismetArrayLibrary.Array_Clear` (`self.DynamicMI`))
  (set `self.OriginalMaterials` (`MeshComponent.GetMaterials` (`self.Mesh`)))
  (for _array_element (`self.FadeMaterialInstance`)
    (bind _returnvalue (`KismetMaterialLibrary.CreateDynamicMaterialInstance` _array_element))
    (`KismetArrayLibrary.Array_AddUnique` (`self.DynamicMI`) _returnvalue)))