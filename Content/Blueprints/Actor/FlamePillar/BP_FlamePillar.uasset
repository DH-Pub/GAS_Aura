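; BP_FlamePillar is a flame pillar actor whose FireLight flickers through a light function material.
; On BeginPlay it creates a dynamic instance of MI_LightFlicker, assigns it to the light and randomizes its RandomShift parameter, so each pillar can flicker out of sync.
; An alternative timeline-driven intensity flicker, randomly playing forward or in reverse, remains in the graph but is disconnected and never runs.
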(event `self.ReceiveBeginPlay`
  (bind _returnvalue (`KismetMaterialLibrary.CreateDynamicMaterialInstance` "/Game/Blueprints/Actor/FlamePillar/MI_LightFlicker.MI_LightFlicker"))
  (`LightComponent.SetLightFunctionMaterial` (`self.FireLight`) _returnvalue)
  (`MaterialInstanceDynamic.SetScalarParameterValue` _returnvalue "RandomShift" (`KismetMathLibrary.RandomFloatInRange` -0.5 0.5)))

(fn `UserConstructionScript`)