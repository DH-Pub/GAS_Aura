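; BP_FireArea is a fire area effect actor that applies a stun to actors when they leave its box.
; Box overlap begin and end events forward to OnOverlap and OnEndOverlap, which are not defined in this graph.
; On exit, it also gives any actor with an Ability System Component a GE_Stun spec, its duration set by caller through the Effect.Duration tag.
; A duplicate stun chain is left unconnected.
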(event `self.Box.OnComponentBeginOverlap`
  (params (OverlappedComponent :type "PrimitiveComponent Object Reference") (OtherActor :type "Actor Object Reference") (OtherComp :type "PrimitiveComponent Object Reference") (OtherBodyIndex :type Integer) (bFromSweep :type Boolean) (SweepResult :type "HitResult Structure (by ref)"))
  (`self.OnOverlap` OtherActor SweepResult))

(event `self.Box.OnComponentEndOverlap`
  (params (OverlappedComponent :type "PrimitiveComponent Object Reference") (OtherActor :type "Actor Object Reference") (OtherComp :type "PrimitiveComponent Object Reference") (OtherBodyIndex :type Integer))
  (bind _returnvalue (`AbilitySystemBlueprintLibrary.GetAbilitySystemComponent` OtherActor))
  (`self.OnEndOverlap` OtherActor)
  (`/Engine/EditorBlueprintResources/StandardMacros.IsValid` _returnvalue
    (:`Is Valid`
      (bind _returnvalue_2 (`AbilitySystemBlueprintLibrary.AssignTagSetByCallerMagnitude` (`AbilitySystemComponent.MakeOutgoingSpec` :`self` _returnvalue :`GameplayEffectClass` "/Game/Blueprints/AbilitySystem/GameplayEffects/Debuff/GE_Stun.GE_Stun_C") (struct :`TagName` "Effect.Duration") 3.0))
      (`AbilitySystemComponent.BP_ApplyGameplayEffectSpecToSelf` _returnvalue _returnvalue_2))))

(fn `UserConstructionScript`)