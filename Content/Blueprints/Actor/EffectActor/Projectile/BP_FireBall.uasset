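; BP_FireBall is a fireball projectile that returns to its instigator like a boomerang after passing its maximum distance.
; The max-distance override clears HitActors, then a timeline lerps it from that point to the instigator's live position.
; Velocity is re-aimed at the instigator at constant speed, and the fireball is destroyed when the timeline finishes.
; An older homing-based return and destroy-on-instigator-hit remain as disconnected nodes; OnHitActor is empty.
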(event `self.OnMaxDistancePassed`
  (bind _returnvalue (`self.GetInstigator`))
  (bind _projectilemovement (`self.ProjectileMovement`))
  (bind _returnvalue_2 (`self.K2_GetActorLocation` _returnvalue))
  (`KismetArrayLibrary.Array_Clear` (`self.HitActors`))
  (set `self.FromLoc` (`self.K2_GetActorLocation`))
  (bind (_direction _percentage) (`Timeline|GoingBack`)
    (:`Update`
      (`/Engine/EditorBlueprintResources/StandardMacros.IsValid` _returnvalue
        (:`Is Valid`
          (`self.K2_SetActorLocation` (`KismetMathLibrary.VLerp` (`self.FromLoc`) _returnvalue_2 _percentage))
          (set `MovementComponent.Velocity` (* (`KismetMathLibrary.Normal` (- _returnvalue_2 (`self.K2_GetActorLocation`))) (`KismetMathLibrary.VSize` (`MovementComponent.Velocity` _projectilemovement))) _projectilemovement))))
    (:`Finished`
      (`self.K2_DestroyActor`))))

(event `self.BP_OnHitActor`
  (params (bIsAlly :type Boolean) (OtherActor :type "Actor Object Reference") (SweepResult :type "HitResult Structure (by ref)")))

(fn `UserConstructionScript`)