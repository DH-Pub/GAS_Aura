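; Anim notify state that switches target tracking on for an Aura character during a window of an animation.
; On begin it casts the mesh owner to AuraCharacterBase, sets its Tracking flag and enables actor tick.
; On end it clears the flag and disables actor tick, so the character ticks only while the window is active.
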(fn `Received_NotifyBegin`
  (params (MeshComp :type "SkeletalMeshComponent Object Reference") (Animation :type "AnimSequenceBase Object Reference") (TotalDuration :type "Float (single-precision)") (EventReference :type "AnimNotifyEventReference Structure (by ref)"))
  (returns (ReturnValue :type Boolean))
  (bind _asaura_character_base (cast `AuraCharacterBase` (`ActorComponent.GetOwner` MeshComp)))
  (bind _output_get (set `AuraCharacterBase.bTracking` true _asaura_character_base))
  (`Actor.SetActorTickEnabled` _asaura_character_base _output_get)
  (return false))

(fn `Received_NotifyEnd`
  (params (MeshComp :type "SkeletalMeshComponent Object Reference") (Animation :type "AnimSequenceBase Object Reference") (EventReference :type "AnimNotifyEventReference Structure (by ref)"))
  (returns (ReturnValue :type Boolean))
  (bind _asaura_character_base (cast `AuraCharacterBase` (`ActorComponent.GetOwner` MeshComp)))
  (bind _output_get (set `AuraCharacterBase.bTracking` false _asaura_character_base))
  (`Actor.SetActorTickEnabled` _asaura_character_base _output_get)
  (return false))