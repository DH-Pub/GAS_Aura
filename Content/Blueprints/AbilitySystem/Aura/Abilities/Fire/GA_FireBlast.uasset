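; Fire Blast gameplay ability for Aura that launches projectiles along the character's capsule forward vector and can be re-triggered mid-flight.
; Activation commits the cost and spawns the projectiles, then waits for a replicated InputPressed event.
; That press forces every spawned projectile past its max travel distance by invalidating the limit and calling OnMaxDistancePassed.
; Cooldown is deferred until OnProjectileDestroyed, which also ends the ability.
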(event `self.K2_ActivateAbility`
  (`self.K2_CommitAbilityCost` false)
  (`AbilityTask_SpawnProjectile.SpawnProjectile` "None" (`SceneComponent.GetForwardVector` (`Character.CapsuleComponent` (`self.AuraCharacter`)))
    (:`OnSpawnFinish`
      (`AT_WaitGenericEvent.WaitGenericReplicatedEvent` "InputPressed"
        (:`OnReceived`
          (for _array_element (`self.ProjectilesSpawned`)
            (set `AuraProjectile.MaxTravelDistance` -1.0 _array_element)
            (`AuraProjectile.OnMaxDistancePassed` _array_element)))))))

(event `self.BP_OnProjectileDestroyed`
  (params (DestroyedProjectile :type "AuraProjectile Object Reference"))
  (`self.K2_CommitAbilityCooldown` false)
  (`self.K2_EndAbility`))