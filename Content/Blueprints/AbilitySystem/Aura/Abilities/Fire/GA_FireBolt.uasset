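; Fire Bolt gameplay ability that casts projectiles from the Weapon socket toward the cursor hit point and target.
; On activation it commits, sends aim data and plays a cast montage, whose gameplay event triggers the projectile spawn.
; Cancellation is locked once the montage starts and restored on ability end.
; Description functions format current and upgrade text with cost, cooldown, projectile count and damage; unconnected test nodes remain in the graph.
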(event `self.K2_ActivateAbility`
  (`self.K2_CommitAbility`)
  (bind (_asynctaskproxy _cursorhit _target) (`AbilityTask_AimData.SendAimData`)
    (:`then`)
    (:`ValidData`
      (`AT_PlayMontageWaitEvent.PlayMontageWaitEvent` "/Game/Blueprints/Character/Aura/AM_Cast_FireBolt.AM_Cast_FireBolt" (struct :`GameplayTags` (struct :`(TagName` "GameplayEventTagsCategory.Montage.1")))
        (:`then`
          (`self.SetCanBeCanceled` false) ; Cannot be canceled until\nprojectile is spawned
        )
        (:`OnCompleted`
          (`self.K2_EndAbility` :!label _label))
        (:`OnBlendOut`
          (goto _label))
        (:`OnInterrupted`
          (goto _label))
        (:`OnCancelled`
          (goto _label))
        (:`EventReceived`
          (`AbilityTask_SpawnProjectile.SpawnProjectile` "Weapon" _cursorhit _target
            (:`OnSpawnFinish`
              (`self.K2_EndAbility`))))))))

(event `self.K2_OnEndAbility`
  (params (bWasCancelled :type Boolean))
  (`self.SetCanBeCanceled` true))

(fn `GetDescription`
  (params (Details :type "AbilityDetails Structure (by ref)"))
  (returns (OutDescription :type Text))
  (bind _returnvalue (`self.GetLevelFromDetails` (`self.Details`)))
  (return (`|FormatText` "FireBolt.Current" Details_Level Details_CostMana Details_BaseCooldown (`self.GetProjectileNumsAtLevel` _returnvalue) (`self.GetDamageAtLevel` _returnvalue))))

(fn `GetLevelChangeDescription`
  (params (Details :type "AbilityDetails Structure (by ref)") (ChangeDetails :type "AbilityDetails Structure (by ref)"))
  (returns (OutDescription :type Text))
  (bind (_level _costmana _costhealth _basecooldown) (break `AbilityDetails` Details))
  (bind (_level_2 _costmana_2 _costhealth_2 _basecooldown_2) (break `AbilityDetails` ChangeDetails))
  (bind _returnvalue (`self.GetLevelFromDetails` (`local.ChangeDetails`)))
  (bind _returnvalue_2 (`self.GetLevelFromDetails` (`local.Details`)))
  (return (`|FormatText` "FireBolt.Upgrade" _level _level_2 _costmana _costmana_2 _basecooldown _basecooldown_2 (`self.GetProjectileNumsAtLevel` _returnvalue_2) (`self.GetProjectileNumsAtLevel` _returnvalue) (`self.GetDamageAtLevel` _returnvalue_2) (`self.GetDamageAtLevel` _returnvalue))))