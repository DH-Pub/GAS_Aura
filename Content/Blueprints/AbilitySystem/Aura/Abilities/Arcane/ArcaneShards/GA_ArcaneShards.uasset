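; Arcane Shards gameplay ability that plays a series of shard gameplay cues around a targeted location.
; It waits on an indicator trace, commits, then spawns a server-only BP_PointCollection there to generate hit points with random yaw.
; A looping timer fires one cue and debug sphere per point, then ends the ability, clearing the timer and destroying the collection.
; No damage is applied in this graph.
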(event `self.K2_ActivateAbility`
  (bind _spawndelta (`self.SpawnDelta`))
  (bind (_asynctaskproxy _data) (`AT_WaitIndicatorTrace.WaitIndicatorTrace` (`self.TargetActorClass`) (make `IndicatorDetails` (`Character.CapsuleComponent` (`self.AuraCharacter`)) "None" 500.0 (struct :`Name` "DungeonMesh")) true "None" null)
    (:`ValidData`
      (bind _returnvalue (`self.K2_CommitAbility`))
      (if _returnvalue
        (bind (_asynctaskproxy_2 _spawnedactor) (`GameplayTask_SpawnActor.SpawnActor` null (`.Location` (break `GATargetData_CommonTarget` _data)) (struct) "/Game/Blueprints/Actor/EffectActor/PointCollection/BP_PointCollection.BP_PointCollection_C" true null)
          (:`Success`
            (bind _aspoint_collection (cast `PointCollection` _spawnedactor))
            (bind _output_get (set `self.PointCollection` _aspoint_collection))
            (bind _outhits (`PointCollection.GetPointsOn` _output_get (`self.NumPoints`) (struct :`Name` "DungeonMesh") (`KismetMathLibrary.RandomFloatInRange` 0.0 360.0) 500.0))
            (set `self.OutHits` _outhits)
            (bind _returnvalue_2 (`KismetSystemLibrary.K2_SetTimerDelegate` (delegate `SpawnShard`) _spawndelta true false (- 0.0 _spawndelta)))
            (set `self.SpawnTimer` _returnvalue_2))
          (:`DidNotSpawn`
            (`self.K2_CancelAbility`)))
        (else
          (`self.K2_CancelAbility` :!label _label))))
    (:`Cancelled`
      (goto _label))))

(event `SpawnShard`
  (bind _output (`|GetArrayItem` (`self.OutHits`) (`self.Count`)))
  (if (< (`self.Count`) (`self.NumPoints`))
    (`self.K2_ExecuteGameplayCueWithParams` (struct :`TagName` "GameplayCue.Spell.ArcaneShards") (`GameplayCueFunctionLibrary.MakeGameplayCueParametersFromHitResult` _output))
    (`KismetSystemLibrary.DrawDebugSphere` (`.ImpactPoint` (`GameplayStatics.BreakHitResult` _output)) 100.0 12 (struct :`R` 1.0 :`G` 1.0 :`B` 1.0 :`A` 1.0) 3.0)
    (`/Engine/EditorBlueprintResources/StandardMacros.IncrementInt` (`self.Count`))
    (else
      (`self.K2_EndAbility`))))

(event `self.K2_OnEndAbility`
  (params (bWasCancelled :type Boolean))
  (`|ExecutionSequence`
    (:`then_0`
      (bind _pointcollection (`self.PointCollection`)
        (:`then`
          (`Actor.K2_DestroyActor` _pointcollection))
        (:`else`)))
    (:`then_1`
      (set `self.Count` 0)
      (`KismetSystemLibrary.K2_ClearAndInvalidateTimerHandle` (`self.SpawnTimer`)))))