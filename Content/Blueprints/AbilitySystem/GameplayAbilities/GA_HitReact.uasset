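; GA_HitReact is a gameplay ability that plays an Aura character's hit reaction and knockback.
; OnHitReact plays the character's HitReactMontage, while Knockback moves the character to a location with a MoveTo root motion force and ignores Pawn collision until the force times out.
; Each branch calls TryEndHitReact with its own State.HitReact tag, PlayMontage or Knockback, when it finishes.
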(event `self.OnHitReact`
  (`AbilityTask_PlayMontageAndWait.CreatePlayMontageAndWaitProxy` "None" (`AuraCharacterBase.HitReactMontage` (`self.AuraCharacter`)) 1.0 "None" false
    (:`OnCompleted`
      _)
    (:`OnBlendOut`
      _)
    (:`OnInterrupted`
      _)
    (:`OnCancelled`
      _))
  (`self.TryEndHitReact` (struct :`TagName` "State.HitReact.PlayMontage")))

(event `self.Knockback`
  (params (ToLocation :type "Vector Structure") (InDuration :type "Float (single-precision)") (bInterrupted :type Boolean))
  (`PrimitiveComponent.SetCollisionResponseToChannel` (`Character.CapsuleComponent` (`self.AuraCharacter`)) "ECC_Pawn" "ECR_Ignore")
  (`AbilityTask_ApplyRootMotionMoveToForce.ApplyRootMotionMoveToForce` "None" ToLocation InDuration false "MOVE_None" false null "ClampVelocity"
    (:`OnTimedOut`
      _)
    (:`OnTimedOutAndDestinationReached`
      _))
  (`PrimitiveComponent.SetCollisionResponseToChannel` (`Character.CapsuleComponent` (`self.AuraCharacter`)) "ECC_Pawn" "ECR_Block")
  (`self.TryEndHitReact` (struct :`TagName` "State.HitReact.Knockback")))